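; BP_LiftBase is a multi-stage lift that players call from a floor or send to a stage through a selection widget.
; Its construction script builds shaft and floor instances per stage, with tagged call boxes and maps linking locations to stages.
; Interact reads component tags to start travel or show the widget.
; Timelines lerp the lift to the mapped position, then swing the doors open and reverse them after a delay.
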(event `self.ReceiveBeginPlay`
  ;[1 1 1] BeginPlay
  (bind _returnvalue (`|CreateWidget` "/Game/Lift/Widget/WBP_StageLift.WBP_StageLift_C" null self))
  (set `self.WBP_Stage` _returnvalue)
  (`TimelineComponent.SetPlayRate` (`self.TL_MoveLift`) (/ 1.0 100.0))
  (bind _returnvalue_2 (`|CreateWidget` "/Game/Lift/Widget/WBP_StageNumber.WBP_StageNumber_C" null self))
  (bind _output_get (set `self.WBP_StageNumber` _returnvalue_2))
  (`WidgetComponent.SetWidget` (`self.Widget`) _output_get))

(event `MoveLift`
  (bind _lift (`self.Lift`))
  (bind _value (`BlueprintMapLibrary.Map_Find` (`self.StageCoords`) (`self.StageNumber`)))
  ;[0 0 0] Lift Up/Down
  (bind (_direction _alpha) (`Timeline|TL_MoveLift` :`NewTime` 1.0 :!via `PlayFromStart` :!label _label)
    (:`Update`
      (bind _returnvalue (`KismetMathLibrary.VLerp` (`SceneComponent.RelativeLocation` _lift) _value _alpha))
      (`SceneComponent.K2_SetRelativeLocation` _lift _returnvalue false false)
      (if (== _returnvalue _value :`ErrorTolerance` 1.0)
        (`TimelineComponent.SetPlayRate` (`self.TL_MoveLift`) 1.0)))
    (:`Finished`
      (`self.Open/Close_Doors` true)
      (`KismetSystemLibrary.Delay` 2.0)
      (`self.Open/Close_Doors` false))))

(event `/Game/FirstPerson/Blueprints/BPI_Interract.Interact`
  (params (InteractedCmpnt :type "ActorComponent Object Reference") (Location :type "Vector Structure") (Interactor :type "Actor Object Reference"))
  ;[0 0 0] Lift Up/Down
  (switch `name` (`|GetArrayItem` (`ActorComponent.ComponentTags` InteractedCmpnt))
    (:`CallLift`
      (set `self.StageNumber` (`BlueprintMapLibrary.Map_Find` (`self.CallCoords`) Location))
      (goto _label :!via `PlayFromStart`))
    (:`WhichStage`
      (`UserWidget.AddToViewport` (`self.WBP_Stage`) 0))))

(event `Open/Close_Doors`
  (params (`Opening?` :type Boolean))
  (bind _sm_doorr (`self.SM_DoorR`))
  (if `Opening?`
    (bind (_direction _newtrack_0) (`Timeline|Timeline` :!via `PlayFromStart` :!label _label_2)
      (:`Update`
        (`SceneComponent.K2_SetRelativeRotation` (`self.SM_DoorL`) (`KismetMathLibrary.RLerp` (`SceneComponent.RelativeRotation` (`self.SM_DoorL`)) (struct :`Yaw` 70.0) _newtrack_0) false false)
        (`SceneComponent.K2_SetRelativeRotation` _sm_doorr (`KismetMathLibrary.RLerp` (`SceneComponent.RelativeRotation` _sm_doorr) (struct :`Yaw` -30.0) _newtrack_0) false false)
        (`KismetSystemLibrary.PrintString` "Hello")))
    (else
      (goto _label_2 :!via `Reverse`))))

(fn `UserConstructionScript`
  (`BlueprintMapLibrary.Map_Clear` (`self.StageCoords`))
  (`BlueprintMapLibrary.Map_Clear` (`self.CallCoords`))
  (for _index (range 1 (+ (`self.NumberOfStage`) 1))
    (bind _returnvalue (* _index (.location (`SceneComponent.GetRelativeTransform` (`self.NextLift`)))))
    (bind _returnvalue_2 (`InstancedStaticMeshComponent.AddInstance` (`self.LiftShaft`) (`KismetMathLibrary.MakeTransform` _returnvalue) false))
    (`BlueprintMapLibrary.Map_Add` (`self.StageCoords`) _returnvalue_2 _returnvalue)
    (`InstancedStaticMeshComponent.AddInstance` (`self.ISM_LiftFloor`) (`KismetMathLibrary.MakeTransform` _returnvalue) false)
    (bind _returnvalue_3 (+ (`SceneComponent.RelativeLocation` (`self.CallLift`)) _returnvalue))
    (`BlueprintMapLibrary.Map_Add` (`self.CallCoords`) _returnvalue_3 _returnvalue_2)
    (bind _returnvalue_4 (`AddComponent|NODE_AddBoxComponent-0` :`RelativeTransform` (`KismetMathLibrary.MakeTransform` _returnvalue_3)))
    (`PrimitiveComponent.SetCollisionResponseToChannel` _returnvalue_4 "ECC_Visibility" "ECR_Block")
    (`BoxComponent.SetBoxExtent` _returnvalue_4 (8.0 8.0 20.0) true)
    (`KismetArrayLibrary.Array_AddUnique` (`ActorComponent.ComponentTags` _returnvalue_4) "CallLift")))